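; BP_OpenHatch is an interactable switch that releases physics puzzle materials held above hatches.
; An overlap volume toggles a flag that gates the Interact input while something is inside it.
; Pressing Interact with the flag set destroys the referenced hatch and three layer actors, letting the held materials drop.
; The overlap events do not filter for the player, so any overlapping actor sets or clears the flag.
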(event `InputAction|Interact`
  (params (Key :type "Key Structure"))
  ; If player is inside the collision zone, they can press 'E' (Interact action) to make the next step occur
  (:`Pressed`
    (if (stale `self.CollisonForInput.OnComponentBeginOverlap` _output_get)
      ; Once the player presses 'E' (Interact) button in the collision zone, destroys the hatches which releases the puzzle oriented physics materials held above them.
      (`self.K2_DestroyActor` (`self.HatchRef`))
      (`self.K2_DestroyActor` (`self.Layer 1`))
      (`self.K2_DestroyActor` (`self.Layer 2`))
      (`self.K2_DestroyActor` (`self.Layer 3`)))))

(event `self.CollisonForInput.OnComponentBeginOverlap`
  (params (OverlappedComponent :type "PrimitiveComponent Object Reference") (OtherActor :type "Actor Object Reference") (OtherComp :type "PrimitiveComponent Object Reference") (OtherBodyIndex :type Integer) (bFromSweep :type Boolean) (SweepResult :type "HitResult Structure (by ref)"))
  ; If player is inside the collision zone, they can press 'E' (Interact action) to make the next step occur
  (bind _output_get (set `self.bCanPressButton` true)))

(event `self.CollisonForInput.OnComponentEndOverlap`
  (params (OverlappedComponent :type "PrimitiveComponent Object Reference") (OtherActor :type "Actor Object Reference") (OtherComp :type "PrimitiveComponent Object Reference") (OtherBodyIndex :type Integer))
  ; If player if is not in the zone, make them unable to press the button.
  (set `self.bCanPressButton` false))

(fn `UserConstructionScript`)